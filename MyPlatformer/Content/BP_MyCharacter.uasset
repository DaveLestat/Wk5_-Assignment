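; Player character Blueprint with jump, movement and look controls, plus simple target, death and level-change rules.
; Movement axes follow the controller's yaw, while look axes feed clamped pitch and yaw input.
; Hit prints the other actor's display name, destroying it if "Sphere" or destroying the character and opening MyLevel1 if "Cone".
; Any actor overlap opens MyLevel2, with no check on the overlapped actor.
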(event `InputAction|Jump`
  (params (Key :type "Key Structure"))
  ;[1 1 1] Jump Function
  (:`Pressed`
    (`self.Jump`)))

(event `InputAxis|MoveForward`
  (params (AxisValue :type "Float (single-precision)"))
  ;[1 1 1] Movement Cluster
  (`self.AddMovementInput` (`KismetMathLibrary.GetForwardVector` (`KismetMathLibrary.MakeRotator` 0.0 0.0 (.yaw (`self.GetControlRotation`)))) AxisValue))

(event `InputAxis|MoveRigth`
  (params (AxisValue :type "Float (single-precision)"))
  ;[1 1 1] Movement Cluster
  (`self.AddMovementInput` (`KismetMathLibrary.GetRightVector` (`KismetMathLibrary.MakeRotator` 0.0 0.0 (.yaw (`self.GetControlRotation`)))) AxisValue))

(event `InputAxis|LookUp/LookDown`
  (params (AxisValue :type "Float (single-precision)"))
  ;[1 1 1] LookAround and TurnAround
  (`self.AddControllerPitchInput` (`KismetMathLibrary.FClamp` AxisValue -1.0)))

(event `InputAxis|LookRigth/LookLeft`
  (params (AxisValue :type "Float (single-precision)"))
  ;[1 1 1] LookAround and TurnAround
  (`self.AddControllerYawInput` (`KismetMathLibrary.FClamp` AxisValue -1.0)))

(event `self.ReceiveHit`
  (params (MyComp :type "PrimitiveComponent Object Reference") (Other :type "Actor Object Reference") (OtherComp :type "PrimitiveComponent Object Reference") (bSelfMoved :type Boolean) (HitLocation :type "Vector Structure") (HitNormal :type "Vector Structure") (NormalImpulse :type "Vector Structure") (Hit :type "HitResult Structure (by ref)"))
  (bind _returnvalue (`KismetSystemLibrary.GetDisplayName` Other))
  (`KismetSystemLibrary.PrintString` _returnvalue)
  (if (`KismetStringLibrary.EqualEqual_StrStr` _returnvalue "Sphere")
    (`self.K2_DestroyActor` Other)
    (`KismetSystemLibrary.PrintString` "Target Destroyed")
    (elif (== _returnvalue "Cone")
      (`self.K2_DestroyActor`)
      (`KismetSystemLibrary.PrintString` "You killed yourself!!!")
      (`GameplayStatics.OpenLevel` "MyLevel1"))))

(event `self.ReceiveActorBeginOverlap`
  (params (OtherActor :type "Actor Object Reference"))
  (`GameplayStatics.OpenLevel` "MyLevel2"))

(fn `UserConstructionScript`)